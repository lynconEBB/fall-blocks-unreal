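; Spleef floor block that turns red and drops away after a player character touches it.
; On the server, the trigger overlap disables its own collision, then chains two timelines: PreFall blends the color, Fall lowers the actor and destroys it.
; Color's OnRep updates a dynamic material instance created at BeginPlay, carrying the warning tint to clients.
; The fall lerps from the current location each update, so motion compounds rather than following the curve directly.
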(event `self.ReceiveBeginPlay`
  (bind _returnvalue (`self.K2_GetActorLocation`))
  (set `self.StartPosition` _returnvalue)
  (set `self.FinalLocation` (+ _returnvalue (0.0 0.0 -200.0)))
  (bind _returnvalue_2 (`PrimitiveComponent.CreateDynamicMaterialInstance` (`self.Box`) 0 "/Game/LevelPrototyping/Materials/MI_PrototypeGrid_Gray.MI_PrototypeGrid_Gray" "None"))
  (set `self.Material` _returnvalue_2))

(event `self.Trigger.OnComponentBeginOverlap`
  (params (OverlappedComponent :type "PrimitiveComponent Object Reference") (OtherActor :type "Actor Object Reference") (OtherComp :type "PrimitiveComponent Object Reference") (OtherBodyIndex :type Integer) (bFromSweep :type Boolean) (SweepResult :type "HitResult Structure (by ref)"))
  (`/Engine/EditorBlueprintResources/ActorMacros.Switch Has Authority`
    (:`Authority`
      (cast `/Game/ThirdPerson/Blueprints/BP_ThirdPersonCharacter` OtherActor)
      (`PrimitiveComponent.SetCollisionEnabled` (`self.Trigger`) "NoCollision")
      (bind (_direction _alpha) (`Timeline|PreFall` :!via `PlayFromStart`)
        (:`Update`
          (set `self.Color` (`KismetMathLibrary.LinearColorLerp` (struct :`R` 0.181164 :`G` 0.181164 :`B` 0.181164 :`A` 1.0) (struct :`R` 0.869792 :`G` 0.067952 :`B` 0.075176 :`A` 1.0) _alpha)))
        (:`Finished`
          (bind (_direction_2 _alpha_2) (`Timeline|Fall` :!via `PlayFromStart`)
            (:`Update`
              (`self.K2_SetActorLocation` (`KismetMathLibrary.VLerp` (`self.K2_GetActorLocation`) (`self.FinalLocation`) _alpha_2) false true))
            (:`Finished`
              (`self.K2_DestroyActor`))))))))

(fn `OnRep_Color`
  (`MaterialInstanceDynamic.SetVectorParameterValue` (`self.Material`) "SurfaceColor" (`self.Color`)))

(fn `UserConstructionScript`)